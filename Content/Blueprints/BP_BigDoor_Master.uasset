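; BP_BigDoor_Master is a double door that swings open when the third-person character enters its Front trigger.
; The overlap fires separate left and right events, each playing a timeline that lerps its pivot's relative yaw through a quarter turn.
; Each timeline update also sets that door's open flag, so later overlaps are ignored once both are set; no closing logic exists.
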(event OnComponentBeginOverlap(Front)
  (params (OverlappedComponent :type Primitive%20Component%20Object%20Reference) (OtherActor :type Actor%20Object%20Reference) (OtherComp :type Primitive%20Component%20Object%20Reference) (OtherBodyIndex :type Integer) (bFromSweep :type Boolean) (SweepResult :type Hit%20Result%20Structure%20%28by%20ref%29))
  ;[1 1 1] Open Doors when Character walks from the front
  (if (not (and (Variables|Default|GetDoor%20L%20Open) (Variables|Default|GetDoor%20R%20Open)))
    (Utilities|Casting|CastToBP_ThirdPersonCharacter OtherActor)
    (CallFunction|OpenDoorL)
    (CallFunction|OpenDoorR)))

(event Custom|OpenDoorL
  ;[1 1 1] Open Left Door
  (bind _doorfloat (Timeline|OpenDoorLeft PlayFromStart)
    (:Update
      (Transformation|SetRelativeRotation (Variables|Default|GetPivotDoorL) (Math|Rotator|MakeRotator 0.0 0.0 (Math|Float|Lerp 0.0 9e+01 _doorfloat)) false false)
      (Variables|Default|SetDoor%20L%20Open true))))

(event Custom|OpenDoorR
  ;[1 1 1] Open Door Right
  (bind _doorfloat (Timeline|OpenDoorRight PlayFromStart)
    (:Update
      (Transformation|SetRelativeRotation (Variables|Default|GetPivotDoorR) (Math|Rotator|MakeRotator 0.0 0.0 (Math|Float|Lerp 0.0 9e+01 _doorfloat)) false false)
      (Variables|Default|SetDoor%20R%20Open true))))

(event EventBeginPlay)

(event Collision|EventActorBeginOverlap
  (params (OtherActor :type Actor%20Object%20Reference)))

(event EventTick
  (params (DeltaSeconds :type Float%20%28single-precision%29)))

(fn ConstructionScript)