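; BP_DoorOneSide is a double door that initially may open only from the back, like a shortcut unlock.
; Interact opens from the front only if OpenSide is true; from the back it always opens, sets OpenSide and updates the front text.
; Timelines drive yaw lerps on both pivots to swing away from the player, though the back path's right-door alpha is fixed at zero.
; No closing logic exists.
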(event EventBeginPlay
  (|CallParentFunction) ; This node is disabled and will not be called.\nDrag off pins to build functionality.
)

(event Collision|EventActorBeginOverlap
  (params (OtherActor :type Actor%20Object%20Reference))
  (|CallParentFunction OtherActor) ; This node is disabled and will not be called.\nDrag off pins to build functionality.
)

(event EventTick
  (params (DeltaSeconds :type Float%20%28single-precision%29))
  (|CallParentFunction DeltaSeconds) ; This node is disabled and will not be called.\nDrag off pins to build functionality.
)

(event EventInteract
  (if (Variables|Default|GetOpenSide)
    (if (Variables|Default|GetIsPlayerInFront)
      (bind _doorfloat (Timeline|Timeline_3 PlayFromStart)
        (:Update
          (Transformation|SetRelativeRotation (Variables|Default|GetPivotDoorL) (Math|Rotator|MakeRotator 0.0 0.0 (Math|Float|Lerp 0.0 9e+01 _doorfloat)) false false)
          (Variables|Default|SetDoor%20L%20Open true)
          (Transformation|SetRelativeRotation (Variables|Default|GetPivotDoorR) (Math|Rotator|MakeRotator 0.0 0.0 (Math|Float|Lerp 0.0 -9e+01 _doorfloat)) false false)
          (Variables|Default|SetDoor%20R%20Open true)))
      (else
        (if (Variables|Default|GetIsPlayerInBack) :!label _label
          (bind _doorfloat_2 (Timeline|Timeline_4 PlayFromStart)
            (:Update
              (Transformation|SetRelativeRotation (Variables|Default|GetPivotDoorL) (Math|Rotator|MakeRotator 0.0 0.0 (Math|Float|Lerp 0.0 -9e+01 _doorfloat_2)) false false)
              (Variables|Default|SetDoor%20L%20Open true)
              (Transformation|SetRelativeRotation (Variables|Default|GetPivotDoorR) (Math|Rotator|MakeRotator 0.0 0.0 (Math|Float|Lerp 0.0 9e+01 0.0)) false false)
              (Variables|Default|SetDoor%20R%20Open true)
              (Variables|Default|SetOpenSide true)
              (Rendering|Components|TextRender|SetText (Variables|Default|GetTextFront) (Variables|Default|GetOpenText)))))))
    (else
      (goto _label))))

(fn ConstructionScript
  (|CallParentFunction))